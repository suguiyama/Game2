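; First-person shooter player Blueprint with mouse look, forward and strafe movement, and reticle and points widgets created on BeginPlay.
; Left click fires a hitscan trace from the camera, rate-limited by a DoOnce reset after a short delay, with timed muzzle flash and gunfire sound.
; Hits on either Barata enemy type apply damage and a physics impulse along the shot, with physics later switched off on the v2 enemy.
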(event `Key|LeftMouseButton`
  (params (Key :type "Key Structure"))
  (bind _muzzleflash (`self.MuzzleFlash`))
  (bind _camera (`self.Camera`))
  (bind _returnvalue (`SceneComponent.K2_GetComponentLocation` _camera))
  (:`Pressed`
    (`|ExecutionSequence`
      (:`then_0`
        ;[1 1 1] Firing logic
        (`/Engine/EditorBlueprintResources/StandardMacros.DoOnce` false :!label _label
          (:`Completed`
            (`|ExecutionSequence`
              (:`then_0`
                (bind _outhit (`KismetSystemLibrary.LineTraceSingle` _returnvalue (+ (* (`KismetMathLibrary.GetForwardVector` (`SceneComponent.K2_GetComponentRotation` _camera)) 20000.0) _returnvalue) "TraceTypeQuery1"))
                (bind (_bblockinghit _binitialoverlap _time _distance _location _impactpoint _normal _impactnormal _physmat _hitactor _hitcomponent _hitbonename _hititem _elementindex _faceindex _tracestart _traceend) (`GameplayStatics.BreakHitResult` _outhit))
                (bind _asenemy_barata (cast `/Game/Enemies/Enemy_Barata` _hitactor)
                  (:`then`
                    (`|ExecutionSequence`
                      (:`then_0`
                        (`GameplayStatics.ApplyDamage` _hitactor 10.0 null null "/Script/Engine.DamageType" :!label _label_2))
                      (:`then_1`
                        (bind _cube (`/Game/Enemies/Enemy_Barata.Cube` _asenemy_barata))
                        (`PrimitiveComponent.SetSimulatePhysics` _cube true)
                        (bind _returnvalue_2 (* (- _traceend _tracestart) 1.0))
                        (`PrimitiveComponent.AddImpulse` _cube _returnvalue_2 "None" false))))
                  (:`CastFailed`
                    (bind _asenemy_baratav_2 (cast `/Game/Enemies/Enemy_Baratav2` _hitactor))
                    (`|ExecutionSequence`
                      (:`then_0`
                        (goto _label_2))
                      (:`then_1`
                        (bind _capsulecomponent (`Character.CapsuleComponent` _asenemy_baratav_2))
                        (`PrimitiveComponent.SetSimulatePhysics` _capsulecomponent true)
                        (`PrimitiveComponent.AddImpulse` _capsulecomponent _returnvalue_2 "None" false)
                        (`KismetSystemLibrary.Delay` 2.0)
                        (`PrimitiveComponent.SetSimulatePhysics` _capsulecomponent false))))))
              (:`then_1`
                (`KismetSystemLibrary.Delay` 0.2)
                (goto _label :!via `Reset`))))))
      (:`then_1`
        ;[1 1 1] Firing VFX
        (`/Engine/EditorBlueprintResources/StandardMacros.DoOnce` false :!label _label_3
          (:`Completed`
            (`|ExecutionSequence`
              (:`then_0`
                (`KismetSystemLibrary.Delay` 0.2)
                (`SceneComponent.SetVisibility` _muzzleflash false false)
                (goto _label_3 :!via `Reset`))
              (:`then_1`
                (`SceneComponent.SetVisibility` _muzzleflash true false))
              (:`then_2`
                (`GameplayStatics.PlaySoundAtLocation` "/Game/Sounds/gunfire.gunfire" (`SceneComponent.K2_GetComponentLocation` _muzzleflash) (struct) 1.0 1.0 0.0 null null null)))))))))

(event `InputAxis|Turn`
  (params (AxisValue :type "Float (single-precision)"))
  ;[1 1 1] Camera
  (`self.AddControllerYawInput` AxisValue))

(event `InputAxis|LookUp`
  (params (AxisValue :type "Float (single-precision)"))
  ;[1 1 1] Camera
  (`self.AddControllerPitchInput` AxisValue))

(event `InputAxis|MoveForward`
  (params (AxisValue :type "Float (single-precision)"))
  ;[1 1 1] Movement
  (`self.AddMovementInput` (`SceneComponent.GetForwardVector` (`self.CapsuleComponent`)) AxisValue))

(event `InputAxis|StrafeRight`
  (params (AxisValue :type "Float (single-precision)"))
  ;[1 1 1] Movement
  (`self.AddMovementInput` (`SceneComponent.GetRightVector` (`self.CapsuleComponent`)) AxisValue))

(event `self.ReceiveBeginPlay`
  (bind _returnvalue (`GameplayStatics.GetPlayerController` 0))
  ;[1 1 1] UI
  (`|ExecutionSequence`
    (:`then_0`
      (bind _returnvalue_2 (`|GenericCreateObject` "/Game/UI/Reticle.Reticle_C" _returnvalue))
      (`UserWidget.AddToViewport` _returnvalue_2 0))
    (:`then_1`
      (bind _returnvalue_3 (`|GenericCreateObject` "/Game/UI/Points.Points_C" _returnvalue))
      (`UserWidget.AddToViewport` _returnvalue_3 0))))

(fn `UserConstructionScript`)